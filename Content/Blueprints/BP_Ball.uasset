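; BP_Ball is a physics ball that caps runaway speed with visual and audio feedback.
; Its particle system starts hidden, and Tick watches the mesh velocity for a high-speed threshold.
; Crossing it shows the particles, then after a brief Delay halves the linear velocity and plays the TooFast sound at the ball.
; The particles are never hidden again once shown.
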(event `self.ReceiveBeginPlay`
  (`SceneComponent.SetVisibility` (`self.ParticleSystem`) false false))

(event `self.ReceiveTick`
  (params (DeltaSeconds :type "Float (single-precision)"))
  (bind _returnvalue (`SceneComponent.GetComponentVelocity` (`self.BallMesh`)))
  (if (>= (`KismetMathLibrary.VSize` _returnvalue) 2000.0)
    (`SceneComponent.SetVisibility` (`self.ParticleSystem`) true false)
    (`KismetSystemLibrary.Delay` 0.05)
    (`PrimitiveComponent.SetAllPhysicsLinearVelocity` (`self.BallMesh`) (/ _returnvalue 2.0) false)
    (`GameplayStatics.PlaySoundAtLocation` "/Game/Sounds/TooFast.TooFast" (`SceneComponent.K2_GetComponentLocation` (`self.BallMesh`)) (struct) 1.0 1.0 0.0 null null null)))

(fn `UserConstructionScript`)