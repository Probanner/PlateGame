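; BP_PlatePawn is the player pawn that handles ball clearing and the death screen.
; Right mouse button destroys every BP_Ball actor in the level.
; On BeginPlay it binds to its ScoreComponent's OnDead event, apparently to run Death, which shows the DeathWidget, switches to UI-only input and reveals the cursor.
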(event `self.ReceiveTick`
  (params (DeltaSeconds :type "Float (single-precision)")))

(event `Key|RightMouseButton`
  (params (Key :type "Key Structure"))
  (:`Pressed`
    (bind _outactors (`GameplayStatics.GetAllActorsOfClass` "/Game/Blueprints/BP_Ball.BP_Ball_C"))
    (for _array_element _outactors
      (`self.K2_DestroyActor` _array_element))))

(event `self.ReceiveBeginPlay`
  (add `ScoreComponent.OnDead` (`self.ScoreComponent`) (`|CreateDelegate` :!event `Death`)))

(event `Death`
  (bind _returnvalue (`GameplayStatics.GetPlayerController` 0))
  (bind _returnvalue_2 (`|CreateWidget` "/Game/Widget/DeathWidget.DeathWidget_C"))
  (`UserWidget.AddToViewport` _returnvalue_2 0)
  (`WidgetBlueprintLibrary.SetInputMode_UIOnlyEx` _returnvalue _returnvalue_2)
  (set `PlayerController.bShowMouseCursor` true _returnvalue))

(fn `UserConstructionScript`)